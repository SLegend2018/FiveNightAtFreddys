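; Game instance for a Doom game that handles multiplayer sessions and holds saved player setup values.
; It creates LAN or Steam sessions through Advanced Sessions, tagged with the host's name and session type, then opens a listen-server level.
; Joining works by console command or accepted invite, and received invites are forwarded to the HUD menu.
; Steam permission, nickname and FrameHate are copied from a save object, which is written to one fixed slot.
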(event Custom|CreateAdvancedSession
  (params (PlayerController :type Player%20Controller%20Object%20Reference) (bUseLan :type Boolean) (LevelName :type Name))
  (bind (_extrasettings _playercontroller _uselan) (CallFunction|SessionConfig PlayerController bUseLan))
  (|AdvancedSession _extrasettings _playercontroller 5 5 _uselan true false true true false false false true
    (:OnSuccess
      (Game|OpenLevel(byName) LevelName true "listen")
      (Viewport|RemoveAllWidgets)
      (Input|SetInputModeGameOnly _playercontroller))
    (:OnFailure
      (Development|PrintString "Failed to create session"))))

(event Custom|JoinSessionByIp
  (params (Command :type String) (PlayerController :type Player%20Controller%20Object%20Reference))
  (Development|ExecuteConsoleCommand Command PlayerController)
  (Viewport|RemoveAllWidgets)
  (Input|SetInputModeGameOnly PlayerController))

(event EventOnSessionInviteReceived
  (params (LocalPlayerNum :type Integer) (PersonInviting :type BP%20Unique%20Net%20Id%20Structure) (AppId :type String) (SessionToJoin :type Blueprint%20Session%20Result%20Structure%20%28by%20ref%29))
  (Default|OnSteamInviteReceived (Variables|/Game/Doom/Hud/MainHUD.MainHUD_C|GetMenuWG (Default|MainHUDReference (CallFunction|GetPlayerController))) LocalPlayerNum PersonInviting AppId SessionToJoin))

(event EventOnSessionInviteAccepted
  (params (LocalPlayerNum :type Integer) (PersonInvited :type BP%20Unique%20Net%20Id%20Structure) (SessionToJoin :type Blueprint%20Session%20Result%20Structure%20%28by%20ref%29))
  (|JoinSession (CallFunction|GetPlayerController) SessionToJoin
    (:OnSuccess
      (Viewport|RemoveAllWidgets)
      (Input|SetInputModeGameOnly (CallFunction|GetPlayerController)))
    (:OnFailure
      (Development|PrintString "Failed to join session"))))

(event Custom|SetCurrentSaveGame
  (params (DoomSaveRef :type DOOM%20Save%20Game%20Object%20Reference))
  (Variables|Default|SetDoomSaveRef DoomSaveRef))

(event Custom|GetSaveData
  (params (DoomSaveRef :type DOOM%20Save%20Game%20Object%20Reference))
  (bind _output_get (Variables|Default|SetDoomSaveRef DoomSaveRef))
  (CallFunction|LoadSave _output_get))

(event Custom|SaveGameToSlot
  (SaveGame|SaveGametoSlot (Variables|Default|GetDoomSaveRef) "DOOM_SaveGame"))

(fn LoadSave
  (params (SaveRef :type DOOM%20Save%20Game%20Object%20Reference))
  (Variables|Network|SetIsSteamAllowed (Variables|/Game/Doom/Blueprint/DOOM_SaveGame.DOOM_SaveGame_C|GetUseSteam? SaveRef))
  (Variables|Network|SetNickname (Variables|/Game/Doom/Blueprint/DOOM_SaveGame.DOOM_SaveGame_C|GetNickname SaveRef))
  (Variables|DisplaySettings|SetFrameHate (Variables|/Game/Doom/Blueprint/DOOM_SaveGame.DOOM_SaveGame_C|GetFrameHate SaveRef)))

(fn SaveSetupValues
  (params (IsSteamAllowed :type Boolean) (Nickname :type Text) (FrameHate :type Float%20%28single-precision%29))
  (Variables|Network|SetIsSteamAllowed IsSteamAllowed)
  (Variables|Network|SetNickname Nickname)
  (Variables|DisplaySettings|SetFrameHate FrameHate))

(fn SessionConfig
  (params (Player%20Controller :type Player%20Controller%20Object%20Reference) (bUseLan :type Boolean))
  (return (Utilities|Array|MakeArray (Class|AdvancedSessionsLibrary|MakeLiteralSessionPropertyString "SessionName" (select bUseLan (Utilities|String|ToString(Text) (Variables|Network|GetNickname)) (Class|AdvancedIdentityLibrary|GetPlayerNickname (Class|AdvancedSessionsLibrary|GetUniqueNetID Player%20Controller)))) (Class|AdvancedSessionsLibrary|MakeLiteralSessionPropertyString "SessionType" (select bUseLan "Lan" "Steam"))) Player%20Controller bUseLan))